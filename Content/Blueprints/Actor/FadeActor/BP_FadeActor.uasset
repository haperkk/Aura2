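; Static mesh actor that fades in and out through a material opacity parameter.
; The construction script caches original materials and builds dynamic instances from a separate fade material list.
; Fadein applies those instances and plays a timeline driving Opacity_Fade, restoring the original materials once the track finishes at full value.
; FadeOut only reverses the timeline, without reapplying the fade instances.
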(event EventBeginPlay)

(event Collision|EventActorBeginOverlap
  (params (OtherActor :type Actor%20Object%20Reference)))

(event EventTick
  (params (DeltaSeconds :type Float%20%28single-precision%29)))

(event EventFadein
  (CallFunction|SetMateialstoDynamicInstance)
  (bind _fadeintrack (Timeline|FadeInTimeline PlayFromStart)
    (:Update
      (for _array_element (Variables|Default|GetDynamicMaterialInstances)
        (Rendering|Material|SetScalarParameterValue _array_element "Opacity_Fade" _fadeintrack :!class /Script/Engine.MaterialInstanceDynamic)))
    (:Finished
      (if (>= _fadeintrack 1.0)
        (CallFunction|ResetMaterials)))))

(event EventFadeOut
  (bind _fadeintrack (Timeline|FadeInTimeline Reverse)
    (:Update
      (for _array_element (Variables|Default|GetDynamicMaterialInstances)
        (Rendering|Material|SetScalarParameterValue _array_element "Opacity_Fade" _fadeintrack :!class /Script/Engine.MaterialInstanceDynamic)))
    (:Finished
      (if (>= _fadeintrack 1.0)
        (CallFunction|ResetMaterials)))))

(fn ConstructionScript
  (Utilities|Array|Clear (Variables|Default|GetDynamicMaterialInstances))
  (Variables|Default|SetOriginalMaterials (Rendering|Material|GetMaterials (Variables|Default|GetStaticMesh)))
  (for _array_element (Variables|Default|GetFadeMatrtials)
    (bind _returnvalue (Rendering|Material|CreateDynamicMaterialInstance _array_element "None" "None" :!class /Script/Engine.KismetMaterialLibrary))
    (Utilities|Array|AddUnique (Variables|Default|GetDynamicMaterialInstances) _returnvalue)))

(fn SetMateialstoDynamicInstance
  (for (_array_element _array_index) (Variables|Default|GetDynamicMaterialInstances)
    (Rendering|Material|SetMaterial (Variables|Default|GetStaticMesh) _array_index _array_element)))

(fn ResetMaterials
  (for (_array_element _array_index) (Variables|Default|GetOriginalMaterials)
    (Rendering|Material|SetMaterial (Variables|Default|GetStaticMesh) _array_index _array_element)))