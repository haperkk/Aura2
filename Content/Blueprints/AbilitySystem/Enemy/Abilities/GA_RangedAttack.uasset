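; Enemy ranged attack gameplay ability that fires a projectile at the avatar's combat target.
; On activation it captures the target's location, turns the avatar toward it through motion-agnostic interface messages, and plays a random tagged attack montage.
; The montage's gameplay event spawns the projectile from the tagged socket toward that captured location, then ends the ability while the montage keeps playing.
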(event Ability|EventActivateAbility
  (bind _returnvalue (Ability|GetAvatarActorfromActorInfo))
  (bind _returnvalue_2 (Class|EnemyInterface|GetCombatTarget(Message) _returnvalue))
  (bind _output_get (Variables|Default|SetTargetLocation (Transformation|GetActorLocation _returnvalue_2)))
  (Class|CombatInterface|UpdateFacingTarget(Message) _returnvalue _output_get)
  (bind _returnvalue_3 (Class|CombatInterface|GetAttackMontages(Message) (Ability|GetAvatarActorfromActorInfo)))
  (bind _output_get_2 (Variables|Default|SetTaggedMontage (Class|AuraDamageGameplayAbility|GetRandomTaggedMontagefromArray _returnvalue_3)))
  (Utilities|IsValid (.Montage (Utilities|Struct|BreakTaggedMontage _output_get_2))
    (:Is%20Valid
      (|PlayMontageandWaitProxy "None" (.Montage (Utilities|Struct|BreakTaggedMontage _output_get_2)) 1.0 "None" false 1.0 0.0
        (:then
          (Ability|Tasks|WaitGameplayEvent (.MontageTag (Utilities|Struct|BreakTaggedMontage _output_get_2)) 0
            (:EventReceived
              (Class|AuraProjectileSpell|SpawnProjectile (Variables|Default|GetTargetLocation) (.SocketTag (Utilities|Struct|BreakTaggedMontage _output_get_2)))
              (Ability|EndAbility))))))
    (:Is%20Not%20Valid
      (Ability|EndAbility))))