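; Enemy melee attack ability that faces the combat target and plays a random tagged attack montage from the avatar.
; A gameplay event matching the montage's tag triggers a small sphere check at that montage's combat socket for live players.
; Non-friendly hits take damage and get a blood effect, and any hit fires one MeleeImpact gameplay cue carrying the montage tag.
; The ability ends after the hit check, or when the montage finishes or is interrupted.
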(event Ability|EventActivateAbility
  (bind _returnvalue (Ability|GetAvatarActorfromActorInfo))
  (bind _returnvalue_2 (Ability|GetAvatarActorfromActorInfo))
  (bind _returnvalue_3 (Ability|GetAvatarActorfromActorInfo))
  (Variables|Default|SetHasHitTarget false)
  (bind _returnvalue_4 (Class|EnemyInterface|GetCombatTarget(Message) _returnvalue_3))
  (Class|CombatInterface|UpdateFacingTarget(Message) _returnvalue_3 (Transformation|GetActorLocation _returnvalue_4))
  (bind _returnvalue_5 (Class|CombatInterface|GetAttackMontages(Message) (Ability|GetAvatarActorfromActorInfo)))
  (bind _output_get (Variables|Default|SetTaggedMontage (Class|AuraDamageGameplayAbility|GetRandomTaggedMontagefromArray _returnvalue_5)))
  (Utilities|IsValid (.Montage (Utilities|Struct|BreakTaggedMontage _output_get))
    (:Is%20Valid
      (|PlayMontageandWaitProxy "None" (.Montage (Utilities|Struct|BreakTaggedMontage _output_get)) 1.0 "None" false 1.0 0.0
        (:then
          (Ability|Tasks|WaitGameplayEvent (.MontageTag (Utilities|Struct|BreakTaggedMontage _output_get)) 0
            (:EventReceived
              (bind _returnvalue_6 (Class|CombatInterface|GetCombatSocketLocation(Message) _returnvalue_2 (.SocketTag (Utilities|Struct|BreakTaggedMontage _output_get))))
              (bind _output_get_2 (Variables|Default|SetHitSocketLocation _returnvalue_6))
              (bind _outoverlappingactors (Class|AuraAbilitySystemLibrary|GetLivePlayerwithRadius _returnvalue_2 (Utilities|Array|MakeArray _returnvalue_2) 45.0 _output_get_2))
              (for _array_element _outoverlappingactors
                (if (Class|AuraAbilitySystemLibrary|IsNotFriend (Ability|GetAvatarActorfromActorInfo) _array_element)
                  (Class|AuraDamageGameplayAbility|CauseDamage _array_element)
                  (Variables|Default|SetHasHitTarget true)
                  (Class|CombatInterface|GetBloodEffect(Message) _array_element)))
              (if (Variables|Default|GetHasHitTarget)
                (bind _returnvalue_7 (Class|EnemyInterface|GetCombatTarget(Message) _returnvalue))
                (Class|GameplayAbility|ExecuteGameplayCuewithParams "(TagName=\"GameplayCue.MeleeImpact\")" (Ability|GameplayCue|MakeGameplayCueParameters :AggregatedSourceTags (GameplayTags|MakeGameplayTagContainerfromTag (.montagetag (Variables|Default|GetTaggedMontage))) :Location (Variables|Default|GetHitSocketLocation) :EffectCauser _returnvalue :SourceObject _returnvalue_7)))
              (Ability|EndAbility))))
        (:OnCompleted
          (Ability|EndAbility :!label _label))
        (:OnInterrupted
          (goto _label))
        (:OnCancelled
          (goto _label))))
    (:Is%20Not%20Valid
      (Ability|EndAbility))))