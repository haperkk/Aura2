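; GA_Electrocute is the Gameplay Ability for a lightning channel held while the input is down.
; It stores the mouse hit and owner references, hides the cursor, faces the target, fires a burst cue and plays the electrocute montage.
; The montage event enters the shock loop, disabling movement and adding a looping cue with the weapon and hit location.
; Input release restores cursor and walking, removes the loop cue and ends the ability.
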(event Ability|EventActivateAbility
  (CallFunction|EnforceImplementsCombatInerface)
  ;[1 1 1] Store Mouse Data Info
  (bind _datahandle (|TargetDataUnderMouse)
    (:ValidData
      (Class|AuraBeamSpell|StoreMouseDataInfo (Ability|TargetData|GetHitResultfromTargetData _datahandle))
      (Class|AuraBeamSpell|StoreOwnerVariables)
      (Utilities|FlowControl|Sequence
        (:then_0
          (Variables|/Script/Engine.PlayerController|SetbShowMouseCursor (Variables|Default|GetOwnerPlayerController) false)
          (CallFunction|UpdateFacingTarget)
          (GameplayCue|ExecuteGameplayCue :GameplayCueTag "(TagName=\"GameplayCue.ShockBurst\")")
          (|PlayMontageandWaitProxy "None" (Variables|Default|GetMontage_Electrocute) 1.0 "None" true 1.0 0.0
            (:then
              (Ability|Tasks|WaitGameplayEvent "(TagName=\"Event.Montage.Electrocute\")" 0 true
                (:EventReceived
                  (CallFunction|InShockLoop)
                  (bind _returnvalue (Class|CombatInterface|GetWeapon(Message) (Ability|GetAvatarActorfromActorInfo)))
                  (GameplayCue|AddGameplayCueOnActor(Looping) (Ability|GetAvatarActorfromActorInfo) "(TagName=\"GameplayCue.ShockLoop\")" (Ability|GameplayCue|MakeGameplayCueParameters :Location (Variables|Default|GetMouseHitLocation) :TargetAttachComponent _returnvalue)))))))
        (:then_1
          (Ability|Tasks|WaitInputRelease false
            (:OnRelease
              (CallFunction|PreparetoEndAbility)
              (Ability|EndAbility))))))))

(fn EnforceImplementsCombatInerface
  (if (not (Utilities|DoesObjectImplementInterface (Ability|GetAvatarActorfromActorInfo) "/Script/Aura.CombatInterface"))
    (Ability|EndAbility)))

(fn PreparetoEndAbility
  (Variables|/Script/Engine.PlayerController|SetbShowMouseCursor (Variables|Default|GetOwnerPlayerController) true)
  (Class|CombatInterface|SetinShockLoop(Message) (Ability|GetAvatarActorfromActorInfo) false)
  (Pawn|Components|CharacterMovement|SetMovementMode (Variables|/Script/Engine.Character|GetCharacterMovement (Variables|Default|GetOwnerPlayerCharacter)) "MOVE_Walking" 0)
  (GameplayCue|RemoveGameplayCue "(TagName=\"GameplayCue.ShockLoop\")"))

(fn InShockLoop
  (Class|CombatInterface|SetinShockLoop(Message) (Ability|GetAvatarActorfromActorInfo) true)
  (Pawn|Components|CharacterMovement|SetMovementMode (Variables|/Script/Engine.Character|GetCharacterMovement (Variables|Default|GetOwnerPlayerCharacter)) "MOVE_None" 0))

(fn UpdateFacingTarget
  (Class|CombatInterface|UpdateFacingTarget(Message) (Ability|GetAvatarActorfromActorInfo) (Variables|Default|GetMouseHitLocation)))